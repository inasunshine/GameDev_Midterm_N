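; BP_AddMecha is a bomb-like hazard that changes player health and explodes on overlap.
; On BeginPlay it caches the player pawn as BP_PersonMidterm.
; Box overlap passes a negative amount to that player's HealthUpdates, without checking what overlapped.
; A separate actor overlap event, gated by DoOnce, spawns an explosion emitter at its location and destroys the actor; the Bomb component's overlap event is empty.
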(event `self.ReceiveBeginPlay`
  (bind _asbp_person_midterm (cast `/Game/Midterm/BP_PersonMidterm` (`GameplayStatics.GetPlayerPawn` 0)))
  (set `self.As BP Person Midterm` _asbp_person_midterm))

(event `self.ReceiveActorBeginOverlap`
  (params (OtherActor :type "Actor Object Reference"))
  (`/Engine/EditorBlueprintResources/StandardMacros.DoOnce` false
    (:`Completed`
      (`GameplayStatics.SpawnEmitterAtLocation` "/Game/StarterContent/Particles/P_Explosion.P_Explosion" (`self.K2_GetActorLocation`))
      (`self.K2_DestroyActor`))))

(event `self.Box.OnComponentBeginOverlap`
  (params (OverlappedComponent :type "PrimitiveComponent Object Reference") (OtherActor :type "Actor Object Reference") (OtherComp :type "PrimitiveComponent Object Reference") (OtherBodyIndex :type Integer) (bFromSweep :type Boolean) (SweepResult :type "HitResult Structure (by ref)"))
  (`/Game/Midterm/BP_PersonMidterm.HealthUpdates` (`self.As BP Person Midterm`) -5.0))

(event `self.Bomb.OnComponentBeginOverlap`
  (params (OverlappedComponent :type "PrimitiveComponent Object Reference") (OtherActor :type "Actor Object Reference") (OtherComp :type "PrimitiveComponent Object Reference") (OtherBodyIndex :type Integer) (bFromSweep :type Boolean) (SweepResult :type "HitResult Structure (by ref)")))

(fn `UserConstructionScript`)