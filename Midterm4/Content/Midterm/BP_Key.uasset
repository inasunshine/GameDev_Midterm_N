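; BP_Key is a colored key pickup that the player collects by interacting with it.
; The construction script sets the sphere to green or red from Selection.
; Interact adds Selection as a string to the player BP_PersonMidterm's Keys array, prints an acquisition message, then destroys the key.
; The message indexes Names by the Add result rather than Selection; an older GM_Midterm-based path remains unconnected.
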(event `self.ReceiveBeginPlay`)

(event `/Game/Midterm/BPI_Interactable.Interact`
  (params (NewParam :type "PrimitiveComponent Object Reference"))
  (bind _asbp_person_midterm (cast `/Game/Midterm/BP_PersonMidterm` (`GameplayStatics.GetPlayerCharacter` 0)))
  (bind _returnvalue (`KismetArrayLibrary.Array_Add` (`/Game/Midterm/BP_PersonMidterm.Keys` _asbp_person_midterm) (`KismetStringLibrary.Conv_IntToString` (`self.Selection`))))
  (`KismetSystemLibrary.PrintString` (`KismetStringLibrary.Concat_StrStr` "Key " (`|GetArrayItem` (`self.Names`) _returnvalue) " Acquired"))
  (`self.K2_DestroyActor`))

(event `self.Capsule.OnComponentBeginOverlap`
  (params (OverlappedComponent :type "PrimitiveComponent Object Reference") (OtherActor :type "Actor Object Reference") (OtherComp :type "PrimitiveComponent Object Reference") (OtherBodyIndex :type Integer) (bFromSweep :type Boolean) (SweepResult :type "HitResult Structure (by ref)")))

(fn `UserConstructionScript`
  (bind _sphere (`self.Sphere`))
  (switch `int` (`self.Selection`)
    (:`0`
      (`PrimitiveComponent.SetMaterial` _sphere 0 "/Game/Midterm/M_Green.M_Green"))
    (:`1`
      (`PrimitiveComponent.SetMaterial` _sphere 0 "/Game/Midterm/M_Red.M_Red"))))