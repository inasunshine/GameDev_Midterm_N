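; BP_Door is a locked door that is removed when interacted with while the game mode's key value matches its KeyNumber.
; It caches GM_Midterm on BeginPlay, then Interact compares Keys to KeyNumber, destroying the actor or printing a wrong-key message.
; The construction script colors the door green or red from KeyNumber.
; A Door_Rotate timeline that lerps the door's location is disconnected and never runs.
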(event `self.ReceiveBeginPlay`
  (bind _asgm_midterm (cast `/Game/Midterm/GM_Midterm` (`GameplayStatics.GetGameMode`)))
  (set `self.As GM Midterm` _asgm_midterm))

(event `/Game/Midterm/BPI_Interactable.Interact`
  (params (NewParam :type "PrimitiveComponent Object Reference"))
  (if (== (`/Game/Midterm/GM_Midterm.Keys` (`self.As GM Midterm`)) (`self.KeyNumber`))
    (`self.K2_DestroyActor`)
    (else
      (`KismetSystemLibrary.PrintString` "You dont have the correct key"))))

(event `self.Box.OnComponentBeginOverlap`
  (params (OverlappedComponent :type "PrimitiveComponent Object Reference") (OtherActor :type "Actor Object Reference") (OtherComp :type "PrimitiveComponent Object Reference") (OtherBodyIndex :type Integer) (bFromSweep :type Boolean) (SweepResult :type "HitResult Structure (by ref)")))

(fn `UserConstructionScript`
  (bind _door (`self.Door`))
  (switch `int` (`self.KeyNumber`)
    (:`0`
      (`PrimitiveComponent.SetMaterial` _door 0 "/Game/Midterm/M_Green.M_Green"))
    (:`1`
      (`PrimitiveComponent.SetMaterial` _door 0 "/Game/Midterm/M_Red.M_Red"))))