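; BP_TrapGas is a gas trap that deals damage over time to the player character while inside its damage box.
; Box overlap begin and end set and clear a timer, with the DOT event applying damage through the player's HealthUpdates.
; It binds to a trap-type dispatcher on BP_PersonMidterm at BeginPlay.
; A matching trap type disarms it by disabling the box's collision and destroying the Gas component.
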(event `self.ReceiveBeginPlay`
  (bind _asbp_person_midterm (cast `/Game/Midterm/BP_PersonMidterm` (`GameplayStatics.GetPlayerCharacter` 0)))
  (bind _output_get (set `self.As BP Person Midterm` _asbp_person_midterm))
  (add `/Game/Midterm/BP_PersonMidterm.DP_TrapType` _output_get (delegate `DP_TrapType`)))

(event `DP_TrapType`
  (params (TrapType :type Byte))
  (if (== TrapType (`self.TrapType`))
    (`PrimitiveComponent.SetCollisionEnabled` (`self.DamageBox`) "NoCollision")
    (`ActorComponent.K2_DestroyComponent` (`self.Gas`))))

(event `self.DamageBox.OnComponentBeginOverlap`
  (params (OverlappedComponent :type "PrimitiveComponent Object Reference") (OtherActor :type "Actor Object Reference") (OtherComp :type "PrimitiveComponent Object Reference") (OtherBodyIndex :type Integer) (bFromSweep :type Boolean) (SweepResult :type "HitResult Structure (by ref)"))
  (if (== OtherActor (`self.As BP Person Midterm`))
    (`KismetSystemLibrary.K2_SetTimer` null "" (`self.DOT_Time`))))

(event `DOT`
  (`/Game/Midterm/BP_PersonMidterm.HealthUpdates` (`self.As BP Person Midterm`) (`self.DOT_Damage`)))

(event `self.DamageBox.OnComponentEndOverlap`
  (params (OverlappedComponent :type "PrimitiveComponent Object Reference") (OtherActor :type "Actor Object Reference") (OtherComp :type "PrimitiveComponent Object Reference") (OtherBodyIndex :type Integer))
  (if (== OtherActor (`self.As BP Person Midterm`))
    (`KismetSystemLibrary.K2_ClearTimer` null "DOT")))

(fn `UserConstructionScript`)