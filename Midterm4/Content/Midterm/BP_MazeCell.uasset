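; BP_MazeCell is a modular maze cell that assembles itself in the construction script, with no active runtime logic.
; GridSize sets the floor footprint and wall thickness, and per-side flags add wall meshes at the cell edges using WallHeigth.
; An optional ceiling adds a centered point light with configurable color when its intensity is positive.
; SizetoCubeScale is the helper that turns dimensions into mesh scales.
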(fn `UserConstructionScript`
  (locals (WallThickness :type "Float (double-precision)" :default 1.0) (WallLenth :type "Float (double-precision)" :default 1.0))
  (bind _gridsize (`self.GridSize`))
  (bind _walllenth (`local.WallLenth`))
  (bind _walllenth_2 (`local.WallLenth`))
  (bind _returnvalue (* (`local.WallLenth`) 0.5))
  (set `local.WallLenth` _gridsize)
  (set `local.WallThickness` (* _gridsize 0.1))
  (`SceneComponent.SetRelativeScale3D` (`self.Floor`) (`self.SizetoCubeScale` (`KismetMathLibrary.MakeVector` _walllenth_2 _walllenth_2 (`local.WallThickness`))))
  (if (`self.WestWall`)
    (`AddComponent|NODE_AddStaticMeshComponent-1` :`RelativeTransform` (`KismetMathLibrary.MakeTransform` (0.0 0.0 0.0) (struct) (`self.SizetoCubeScale` (`KismetMathLibrary.MakeVector` (`local.WallLenth`) (`local.WallThickness`) (`self.WallHeigth`))))))
  (if (`self.SouthWall`)
    (`AddComponent|NODE_AddStaticMeshComponent-2` :`RelativeTransform` (`KismetMathLibrary.MakeTransform` (0.0 0.0 0.0) (struct) (`self.SizetoCubeScale` (`KismetMathLibrary.MakeVector` (`local.WallThickness`) (`local.WallLenth`) (`self.WallHeigth`))))))
  (if (`self.NorthWAll`)
    (`AddComponent|NODE_AddStaticMeshComponent-3` :`RelativeTransform` (`KismetMathLibrary.MakeTransform` (`KismetMathLibrary.MakeVector` (- (`local.WallLenth`) (`local.WallThickness`))) (struct) (`self.SizetoCubeScale` (`KismetMathLibrary.MakeVector` (`local.WallThickness`) (`local.WallLenth`) (`self.WallHeigth`))))))
  (if (`self.EastWall`)
    (`AddComponent|NODE_AddStaticMeshComponent-4` :`RelativeTransform` (`KismetMathLibrary.MakeTransform` (`KismetMathLibrary.MakeVector` 0.0 (- (`local.WallLenth`) (`local.WallThickness`))) (struct) (`self.SizetoCubeScale` (`KismetMathLibrary.MakeVector` (`local.WallLenth`) (`local.WallThickness`) (`self.WallHeigth`))))))
  (if (`self.Ceiling`)
    (`AddComponent|NODE_AddStaticMeshComponent-5` :`RelativeTransform` (`KismetMathLibrary.MakeTransform` (`KismetMathLibrary.MakeVector` 0.0 0.0 (`self.WallHeigth`)) (struct) (`self.SizetoCubeScale` (`KismetMathLibrary.MakeVector` _walllenth _walllenth (`local.WallThickness`)))))
    (if (> (`self.LightIntensity`) 0.0)
      (bind _returnvalue_2 (`AddComponent|NODE_AddPointLightComponent-0` :`RelativeTransform` (`KismetMathLibrary.MakeTransform` (`KismetMathLibrary.MakeVector` _returnvalue _returnvalue (* (`self.WallHeigth`) 0.9)))))
      (`LightComponent.SetLightColor` _returnvalue_2 (`self.LightColor`) true)
      (`LightComponent.SetIntensity` _returnvalue_2 (`self.LightIntensity`)))))