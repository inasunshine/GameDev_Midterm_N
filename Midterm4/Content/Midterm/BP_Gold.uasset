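; BP_Gold is a gold pickup that adds its value to the player's gold in GM_Midterm when interacted with, then prints the total and destroys itself.
; The construction script rolls a random value and uses the CreateMesh helper at value thresholds to add randomly offset and scaled meshes, so richer piles show more pieces.
; BeginPlay caches the game mode and shows the value on a text render.
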(event `self.ReceiveBeginPlay`
  (bind _asgm_midterm (cast `/Game/Midterm/GM_Midterm` (`GameplayStatics.GetGameMode`)))
  (set `self.As GM Midterm` _asgm_midterm)
  (`TextRenderComponent.K2_SetText` (`self.TextRender`) (`KismetTextLibrary.Conv_IntToText` (`self.ItemGold`))))

(event `/Game/Midterm/BPI_Interactable.Interact`
  (params (NewParam :type "PrimitiveComponent Object Reference"))
  (bind _output_get (set `/Game/Midterm/GM_Midterm.PlayerGold` (+ (`/Game/Midterm/GM_Midterm.PlayerGold` (`self.As GM Midterm`)) (`self.ItemGold`)) (`self.As GM Midterm`)))
  (`KismetSystemLibrary.PrintString` (`KismetStringLibrary.Concat_StrStr` "Current Gold: " (`KismetStringLibrary.Conv_IntToString` _output_get)))
  (`self.K2_DestroyActor`))

(fn `UserConstructionScript`
  (bind _itemgold (`self.ItemGold`))
  (set `self.ItemGold` (`KismetMathLibrary.RandomIntegerInRange` 1 99))
  (`self.CreateMesh` (>= _itemgold 76)
    (:`then`
      _)
    (:`false`
      _))
  (`self.CreateMesh` (>= _itemgold 26)
    (:`then`
      _)
    (:`false`
      _))
  (`self.CreateMesh` (>= _itemgold 1)))