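; BP_Switch is an interactable switch in the Midterm game that turns off traps of a selected type.
; On BeginPlay it caches the BP_PersonMidterm player character and shows its TrapType enum name on a text render component.
; Interact passes that TrapType to the player's CallDPTrapType, so the player relays the trap change, then prints a debug message.
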(event `self.ReceiveBeginPlay`
  (bind _asbp_person_midterm (cast `/Game/Midterm/BP_PersonMidterm` (`GameplayStatics.GetPlayerCharacter` 0)))
  (set `self.As BP Person Midterm` _asbp_person_midterm)
  (`TextRenderComponent.K2_SetText` (`self.TextRender`) (`KismetTextLibrary.Conv_StringToText` (`|GetEnumeratorNameAsString` (`self.Trap Type`)))))

(event `/Game/Midterm/BPI_Interactable.Interact`
  (params (NewParam :type "PrimitiveComponent Object Reference"))
  (`/Game/Midterm/BP_PersonMidterm.DP_TrapType` (`self.As BP Person Midterm`) (`self.Trap Type`))
  (`KismetSystemLibrary.PrintString` "Turn off Trap"))

(fn `UserConstructionScript`)